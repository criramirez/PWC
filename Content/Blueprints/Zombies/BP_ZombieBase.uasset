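; BP_ZombieBase is a zombie enemy character with health, damage handling and an overhead health bar.
; Construction sets its walk speed from Velocidad and stores the starting health.
; Each Tick updates the bar's percentage and yaws the widget toward the player's follow camera.
; PasarDaño subtracts damage and, on death, detaches the controller, plays the death animation and destroys the actor after five seconds.
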(event EventBeginPlay)

(event Collision|EventActorBeginOverlap
  (params (OtherActor :type Actor%20Object%20Reference)))

(event EventTick
  (params (DeltaSeconds :type Float%20%28single-precision%29))
  ;[1 1 1] Flujo de widget de vida
  (bind _asw_barra_vida_enemigo (Utilities|Casting|CastToW_BarraVidaEnemigo (UserInterface|GetUserWidgetObject (Variables|Default|GetWidget))))
  (Progress|SetPercent (Variables|/Game/Blueprints/Zombies/W_BarraVidaEnemigo.W_BarraVidaEnemigo_C|GetProgressBar_134 _asw_barra_vida_enemigo) (/ (Variables|Default|Getsalud) (Variables|Default|GetsaludInicial)))
  (bind _asbp_jugador (Utilities|Casting|CastToBP_Jugador (Game|GetPlayerCharacter 0)))
  (Transformation|SetWorldRotation (Variables|Default|GetWidget) (Math|Rotator|MakeRotator 0.0 0.0 (.Yaw (Math|Rotator|BreakRotator (Math|Rotator|FindLookatRotation (Transformation|GetWorldLocation (Variables|Default|GetWidget)) (Transformation|GetWorldLocation (Variables|/Game/ThirdPersonBP/Blueprints/BP_Jugador.BP_Jugador_C|GetFollowCamera _asbp_jugador)))))) false false))

(event EventPasarDaño
  (params (dañoRealizado :type Float%20%28single-precision%29))
  (CallFunction|CalcularSalud dañoRealizado)
  (if (Variables|Default|GetestaMuerto?)
    (Class|Pawn|DetachfromControllerPendingDestroy)
    (Components|Animation|PlayAnimation (Variables|Character|GetMesh) "/Game/Blueprints/Zombies/MESH_ZombieBase/Animaciones/zombie_death.zombie_death" false)
    (Utilities|FlowControl|Delay 5.0)
    (Actor|DestroyActor)))

(fn ConstructionScript
  (Variables|/Script/Engine.CharacterMovementComponent|SetMaxWalkSpeed (Variables|Character|GetCharacterMovement) (Variables|Default|Getvelocidad))
  (Variables|Default|SetsaludInicial (Variables|Default|Getsalud)))

(fn CalcularSalud
  (params (daño :type Float%20%28single-precision%29))
  (Variables|Default|Setsalud (- (Variables|Default|Getsalud) daño))
  (Variables|Default|SetestaMuerto? (<= (Variables|Default|Getsalud) 0.0)))