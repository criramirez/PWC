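; Interactable ammo pickup (Municion) in the Zombies folder that shows a HUD message while something overlaps its capsule.
; Overlap begin enables input for player controller 0 and sends the Mensaje text to HUD_Principal; overlap end disables input and clears it.
; Pressing Interactuar destroys the actor without granting any ammo here.
; The overlapping actor is never checked, so any overlap triggers the prompt.
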(event OnComponentBeginOverlap(Capsule)
  (params (OverlappedComponent :type Primitive%20Component%20Object%20Reference) (OtherActor :type Actor%20Object%20Reference) (OtherComp :type Primitive%20Component%20Object%20Reference) (OtherBodyIndex :type Integer) (bFromSweep :type Boolean) (SweepResult :type Hit%20Result%20Structure%20%28by%20ref%29))
  (bind _returnvalue (Game|GetPlayerController 0))
  (Utilities|FlowControl|Sequence
    (:then_0
      (Input|EnableInput _returnvalue))
    (:then_1
      (bind _ashud_principal (Utilities|Casting|CastToHUD_Principal (HUD|GetHUD _returnvalue)))
      (Default|MostarMensaje _ashud_principal true (Variables|Default|GetMensaje)))))

(event OnComponentEndOverlap(Capsule)
  (params (OverlappedComponent :type Primitive%20Component%20Object%20Reference) (OtherActor :type Actor%20Object%20Reference) (OtherComp :type Primitive%20Component%20Object%20Reference) (OtherBodyIndex :type Integer))
  (bind _returnvalue (Game|GetPlayerController 0))
  (Utilities|FlowControl|Sequence
    (:then_0
      (Input|DisableInput _returnvalue))
    (:then_1
      (bind _ashud_principal (Utilities|Casting|CastToHUD_Principal (HUD|GetHUD _returnvalue)))
      (Default|MostarMensaje _ashud_principal false))))

(event EventBeginPlay)

(event Collision|EventActorBeginOverlap
  (params (OtherActor :type Actor%20Object%20Reference)))

(event EventTick
  (params (DeltaSeconds :type Float%20%28single-precision%29)))

(event Input|ActionEvents|InputActionInteractuar
  (params (Key :type Key%20Structure :default "AnyKey"))
  (:Pressed
    (Actor|DestroyActor)))

(fn ConstructionScript)