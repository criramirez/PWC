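; AI controller for zombie enemies that runs the BT_Enemigos behavior tree when it possesses a BP_ZombieBase pawn.
; Its AI Perception update writes whether the player (BP_Jugador) is currently sensed to the "puedoVerJugador?" Blackboard key.
; A collapsed graph holds empty events plus unconnected leftovers of a timer-driven AIMoveTo chase, which never run.
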(event OnTargetPerceptionUpdated(AIPerception)
  (params (Actor :type Actor%20Object%20Reference) (Stimulus :type AI%20Stimulus%20Structure))
  (Utilities|Casting|CastToBP_Jugador Actor)
  (AI|Components|Blackboard|SetValueasBool (AI|GetBlackboard 0) (Utilities|Name|MakeLiteralName "puedoVerJugador?") (.bSuccessfullySensed (Utilities|Struct|BreakAIStimulus Stimulus))))

(event EventOnPossess
  (params (PossessedPawn :type Pawn%20Object%20Reference))
  (Utilities|Casting|CastToBP_ZombieBase PossessedPawn)
  (AI|RunBehaviorTree "/Game/Blueprints/Zombies/BT_Enemigos.BT_Enemigos"))

(fn ConstructionScript)

(event Custom|BuscarAlJugador)

(event EventBeginPlay)